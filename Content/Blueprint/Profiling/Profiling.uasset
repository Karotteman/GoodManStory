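; Profiling helper Blueprint that wraps console commands for debugging and measuring performance.
; Its functions toggle stat displays for frame timing, FPS and scene rendering, and start or stop stat file recordings.
; Others build commands for a range-checked screen percentage and for view modes, mapping the enum through a string array.
; Recap functions open Unreal documentation and a profiling video in the browser.
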(fn `FPS`
  ;[1 1 1] Show a FPS counter and the time to make a frame.
  (`KismetSystemLibrary.ExecuteConsoleCommand` null "stat FPS" null))

(fn `RecapProfiling`
  (`KismetSystemLibrary.LaunchURL` "https://www.youtube.com/watch?v=hcxetY8g_fs"))

(fn `RecapStat`
  (`KismetSystemLibrary.LaunchURL` "https://docs.unrealengine.com/en-us/Engine/Performance/StatCommands"))

(fn `RecapViewMode`
  (`KismetSystemLibrary.LaunchURL` "https://docs.unrealengine.com/en-us/Engine/UI/LevelEditor/Viewports/ViewModes"))

(fn `SceneRendereing`
  ;[1 1 1] Breaks down each part of the rendering.
  (`KismetSystemLibrary.ExecuteConsoleCommand` null "stat SceneRendering" null))

(fn `ScreenPercentage`
  (params (Percent :type Integer :default 10))
  ;[1 1 1] Scale the percent of pixels used.
  (if (`KismetMathLibrary.InRange_IntInt` Percent 10 100)
    (`KismetSystemLibrary.ExecuteConsoleCommand` null (`KismetStringLibrary.BuildString_Int` "" "r.ScreenPercentage " Percent) null)))

(fn `ShowStat`
  (params (withGraph :type Boolean :default true))
  ;[1 1 1] Show the stats.
  ; Indicates the time of each part for a frame.
  (`KismetSystemLibrary.ExecuteConsoleCommand` null "stat unit" null)
  (if withGraph
    (`KismetSystemLibrary.ExecuteConsoleCommand` null "stat unitgraph" null)))

(fn `StartProfiling`
  ;[1 1 1] Start to record a profiling session. Need to be stop with StopProfiling.
  (`KismetSystemLibrary.ExecuteConsoleCommand` null "stat StartFile" null))

(fn `StopProfiling`
  ;[1 1 1] Stop the recording started with StartProfiling.
  (`KismetSystemLibrary.ExecuteConsoleCommand` null "stat StopFile" null))

(fn `ViewMode`
  (params (Mode :type "/Game/EViewMode Enum" :default "NewEnumerator0"))
  (locals (ViewModeString :type "Array of String"))
  ;[1 1 1] Change the view mode.
  ; You can see all the mode in EViewMode.
  ; This modes are useful for debuging/profiling.
  (`KismetSystemLibrary.ExecuteConsoleCommand` null (`KismetStringLibrary.BuildString_Name` "" "" "viewmode " (`|GetArrayItem` (`local.ViewModeString`) (`KismetMathLibrary.Conv_ByteToInt` Mode))) null))