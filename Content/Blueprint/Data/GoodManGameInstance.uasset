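; GoodManGameInstance is the game instance that holds player control settings and a veterancy score for the game.
; ApplyModifsSettings copies look sensitivity and axis inversion onto the current PlayerBlueprint character.
; ComputePlayerVeterancy subtracts a time term, level duration minus its limit, and a lost-life percentage from veterancy, so finishing early earns a bonus.
; It prints the score and penalties on screen for debugging.
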(event `ApplyModifsSettings`
  (bind _asplayer_blueprint (cast `/Game/Blueprint/Character/Players/PlayerBlueprint` (`GameplayStatics.GetPlayerCharacter` 0)))
  (set `BasePlayer.Sensibility` (`self.Sensibility`) _asplayer_blueprint)
  (set `BasePlayer.bInvertedAxisX` (`self.bInvertAxeX`) _asplayer_blueprint)
  (set `BasePlayer.bInvertedAxisY` (`self.bInvertAxeY`) _asplayer_blueprint))

(fn `ComputePlayerVeterancy`
  (locals (TimePenalty :type Integer) (LifePenalty :type Integer))
  (bind _lifepenalty (`local.LifePenalty`))
  (bind _timepenalty (`local.TimePenalty`))
  ;[1 1 1] Apply excess time penalty or bonus
  (set `local.TimePenalty` (`KismetMathLibrary.FTrunc` (- (`self.PlayerLevelDuration`) (`self.LevelDurationLimite`))))
  ;[1 1 1] Apply life loose penalty
  (bind _asbase_player (cast `BasePlayer` (`GameplayStatics.GetPlayerCharacter` 0)))
  (set `local.LifePenalty` (`KismetMathLibrary.FTrunc` (* (- 1.0 (`BaseCharacter.GetLifeRatio` _asbase_player)) 100.0)))
  ;[1 1 1] Apply result
  (bind _output_get (set `self.PlayerVeterancy ` (- (`self.PlayerVeterancy `) (`KismetMathLibrary.Conv_IntToDouble` (+ (`local.TimePenalty`) (`local.LifePenalty`))))))
  ;[1 1 1] Debug
  (`KismetSystemLibrary.PrintString` (`KismetStringLibrary.Concat_StrStr` "PlayerVeterancy : " (`KismetStringLibrary.Conv_DoubleToString` _output_get) " | TimePenalty : " (`KismetStringLibrary.Conv_IntToString` _timepenalty) " | LifePenalty : " (`KismetStringLibrary.Conv_IntToString` _lifepenalty) "| PenaltyTotal : " (`KismetStringLibrary.Conv_IntToString` (+ _timepenalty _lifepenalty))) true true (struct :`R` 0.807764 :`B` 0.841667 :`A` 1.0) 10.0))