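; BloodScreen Blueprint that shows a screen-space blood overlay as damage feedback.
; On BeginPlay it creates the BloodScreenEffect widget, adds it to the viewport and hides its image.
; DisplayDamage adds damage scaled by HitStrength to a target Opacity.
; Tick lerps the image opacity toward that target using delta time as alpha, then decays the target at a rate set by HitRecovery, flooring it at zero.
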(event `self.ReceiveBeginPlay`
  (bind _returnvalue (`|CreateWidget` "/Game/Blueprint/GUI/HUD/BloodScreenEffect.BloodScreenEffect_C"))
  (bind _output_get (set `self.BloodScreenHUD` _returnvalue))
  (`UserWidget.AddToViewport` _output_get 0)
  (`Image.SetOpacity` (`/Game/Blueprint/GUI/HUD/BloodScreenEffect.BloodScreenImage` (`self.BloodScreenHUD`)) 0.0))

(event `self.ReceiveTick`
  (params (DeltaSeconds :type "Float (single-precision)"))
  (bind _bloodscreenimage (`/Game/Blueprint/GUI/HUD/BloodScreenEffect.BloodScreenImage` (`self.BloodScreenHUD`)))
  (bind (_colorandopacity_r _colorandopacity_g _colorandopacity_b _colorandopacity_a) (break `LinearColor` (`Image.ColorAndOpacity` _bloodscreenimage)))
  ;[1 1 1] Lerp to the new opacity
  (`Image.SetOpacity` _bloodscreenimage (`KismetMathLibrary.Lerp` _colorandopacity_a (`self.Opacity`) DeltaSeconds))
  (bind _output_get (set `self.Opacity` (- (`self.Opacity`) (/ DeltaSeconds (`self.HitRecovery`)))))
  (if (< _output_get 0.0)
    (set `self.Opacity` 0.0)))

(fn `DisplayDamage`
  (params (DamageTake :type "Float (double-precision)"))
  (set `self.Opacity` (+ (* DamageTake (`self.HitStrength`)) (`self.Opacity`))))