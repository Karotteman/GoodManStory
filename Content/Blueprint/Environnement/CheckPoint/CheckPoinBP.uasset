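; Checkpoint actor that registers itself as the current checkpoint and respawns the player at its location.
; Active stores the checkpoint in GoodManGameInstance as CurrentCheckPoint.
; RespawnPlayer calls TakeLife on the BasePlayer with its maximum life, moves it to the checkpoint without sweeping, then has EnemiesManager reset the current wave.
; Both functions are invoked externally, as the event graph holds only disabled placeholder events.
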(fn `Active`
  (bind _asgood_man_game_instance (cast `/Game/Blueprint/Data/GoodManGameInstance` (`GameplayStatics.GetGameInstance`)))
  (set `/Game/Blueprint/Data/GoodManGameInstance.CurrentCheckPoint` self _asgood_man_game_instance))

(fn `RespawnPlayer`
  (bind _asbase_player (cast `BasePlayer` (`GameplayStatics.GetPlayerCharacter` 0)))
  (`BaseCharacter.TakeLife` _asbase_player (`BaseCharacter.LifeMax` _asbase_player))
  (`self.K2_SetActorLocation` _asbase_player (`self.K2_GetActorLocation`) false false)
  (`EnemiesManager.ResetCurrentWave` (`self.EnemiesManager`)))

(fn `UserConstructionScript`)