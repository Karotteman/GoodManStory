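; Checkpoint actor that registers itself as the current respawn point and brings the player back to its location.
; Active stores the checkpoint in GoodManGameInstance as CurrentCheckPoint.
; RespawnPlayer calls TakeLife with the player's max life, teleports them to the checkpoint and stops their movement.
; It then resets the EnemiesManager's current wave if CanRestartWave is set, printing a message when the manager reference is missing.
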(fn `Active`
  (bind _asgood_man_game_instance (cast `/Game/Blueprint/Data/GoodManGameInstance` (`GameplayStatics.GetGameInstance`))
    (:`then`
      (set `/Game/Blueprint/Data/GoodManGameInstance.CurrentCheckPoint` self _asgood_man_game_instance))
    (:`CastFailed`
      (`KismetSystemLibrary.PrintString` "Fail to cast gameInstance in CheckPoint"))))

(fn `RespawnPlayer`
  (bind _enemiesmanager (`self.EnemiesManager`))
  (bind _asbase_player (cast `BasePlayer` (`GameplayStatics.GetPlayerCharacter` 0)))
  (`BaseCharacter.TakeLife` _asbase_player (`BaseCharacter.LifeMax` _asbase_player))
  (`self.K2_SetActorLocation` _asbase_player (`self.K2_GetActorLocation`) false true)
  (`MovementComponent.StopMovementImmediately` (`Character.CharacterMovement` _asbase_player))
  (`/Engine/EditorBlueprintResources/StandardMacros.IsValid` _enemiesmanager
    (:`Is Valid`
      (if (`self.CanRestartWave`)
        (`EnemiesManager.ResetCurrentWave` _enemiesmanager)))
    (:`Is Not Valid`
      (`KismetSystemLibrary.PrintString` (`KismetStringLibrary.Concat_StrStr` "EnemiesManager Ref mising in " (`KismetSystemLibrary.GetObjectName` self))))))

(fn `UserConstructionScript`)