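; Boss fireball Blueprint that supplies the audio, visual and haptic feedback for a fireball projectile.
; On BeginPlay it binds to its spawn, destroy, hit-actor and hit-player dispatchers; movement and hit detection are not in this graph.
; Spawn plays a launch sound, and destroy plays an impact sound with a shockwave emitter, both with debug prints.
; Player hits trigger camera shake and controller rumble, while the hit-actor handler is empty.
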(event `self.ReceiveBeginPlay`
  (`|ExecutionSequence`
    (:`then_0`
      ;[1 1 1] Bind event to the callback
      (add `self.OnFireBallSpawn` (delegate `OnFireBallSpawn_Event_0`)))
    (:`then_1`
      (add `self.OnFireBallDestroy` (delegate `OnFireBallDestroy_Event_0`)))
    (:`then_2`
      (add `self.OnFireBallHitActor` (delegate `OnFireBallHitActor_Event_0`)))
    (:`then_3`
      (add `self.OnFireBallHitPlayer` (delegate `OnFireBallHitPlayer_Event_0`)))))

(event `OnFireBallSpawn_Event_0`
  ;[1 1 1] Bind event to the callback
  ;;[0 1 0] OnFire ball spawn
  (`KismetSystemLibrary.PrintString` "FireBall spawn")
  (`GameplayStatics.PlaySoundAtLocation` "/Game/Assets/Sounds/Ennemis/Boss/FireballSounds/Fireball/BossFireballProjectile01.BossFireballProjectile01" (`self.K2_GetActorLocation`) (struct) 1.0 1.0 0.0 "/Game/Blueprint/Audio/FireBallSoundAttenuation.FireBallSoundAttenuation" null self))

(event `OnFireBallDestroy_Event_0`
  (bind _returnvalue (`self.K2_GetActorLocation`))
  ;[1 1 1] Bind event to the callback
  ;;[0 1 0] OnFireBall destroy
  (`KismetSystemLibrary.PrintString` "FireBall destroy")
  (`GameplayStatics.PlaySoundAtLocation` "/Game/Assets/Sounds/Ennemis/Boss/FireballSounds/Fireball/BossFireballProjectileImpact01.BossFireballProjectileImpact01" _returnvalue (struct) 1.0 1.0 0.0 "/Game/Blueprint/Audio/FireBallImpactSoundAttenuation.FireBallImpactSoundAttenuation" null self)
  (`GameplayStatics.SpawnEmitterAtLocation` "/Game/Assets/FX/FXVarietyPack/Particles/P_ky_shotShockwave.P_ky_shotShockwave" _returnvalue (`self.K2_GetActorRotation`) (`self.GetActorScale3D`)))

(event `OnFireBallHitActor_Event_0` :!signature `self.OnFireBallHitActor`
  (params (ActorHit :type "Actor Object Reference"))
  ;[1 1 1] Bind event to the callback
  ;;[0 1 0] OnFire ball hit actor
)

(event `OnFireBallHitPlayer_Event_0` :!signature `self.OnFireBallHitPlayer`
  (params (Player :type "BasePlayer Object Reference"))
  ;[1 1 1] Bind event to the callback
  ;;[0 1 0] OnFire ball hit player
  (`GameplayStatics.PlayWorldCameraShake` "/Game/Blueprint/FX/BaseCameraShake.BaseCameraShake_C" (`self.K2_GetActorLocation` Player) 0.0 3000.0)
  (`PlayerController.PlayDynamicForceFeedback` (`GameplayStatics.GetPlayerController` 0) 1.0 1.0 true false true false))

(fn `UserConstructionScript`)