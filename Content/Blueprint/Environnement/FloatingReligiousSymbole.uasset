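; Environment actor for a religious symbol that stays idle, with Tick disabled, until its Active function is called.
; Active enables Tick, offsets the actor from its mesh's world position by ActivateLocation, applies ActivateRotation and toggles a particle system.
; Tick then plays the Movement timeline, whose track scaled by Amplitude is added to the mesh's current position on each update, producing the floating motion.
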(event `self.ReceiveBeginPlay`
  (`self.SetActorTickEnabled` false))

(event `self.ReceiveTick`
  (params (DeltaSeconds :type "Float (single-precision)"))
  (bind (_direction _newtrack_0) (`Timeline|Movement`)
    (:`Update`
      (`self.K2_SetActorLocation` (+ (* _newtrack_0 (`self.Amplitude`)) (`SceneComponent.K2_GetComponentLocation` (`self.StaticMeshComponent`)))))))

(fn `Active`
  (`self.SetActorTickEnabled` true)
  (`self.K2_SetActorLocationAndRotation` (+ (`self.ActivateLocation`) (`SceneComponent.K2_GetComponentLocation` (`self.StaticMeshComponent`))) (`self.ActivateRotation`))
  (`ActorComponent.ToggleActive` (`self.ParticleSystem1`)))

(fn `UserConstructionScript`)