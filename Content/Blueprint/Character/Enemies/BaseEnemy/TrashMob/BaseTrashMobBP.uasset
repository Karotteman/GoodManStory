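; Base Blueprint for trash mob enemies, defining the shared reactions to character life-cycle events.
; BeginPlay binds handlers to the damage, death, destroy, spawn and life-gain delegates.
; Only the damage handler has logic, triggering a blood splat through the blood particle emitter component; the others are empty stubs.
; The construction script just runs the parent's.
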(event `self.ReceiveBeginPlay`
  (`|ExecutionSequence`
    (:`then_0`
      ;[1 1 1] Define the Trash behaviours
      (`|ExecutionSequence`
        (:`then_0`
          (add `BaseCharacter.OnCharacterTakeDamage` (delegate `OnCharacterTakeDamage_Event_2`)))
        (:`then_1`
          (add `BaseCharacter.OnCharacterDeath` (delegate `OnCharacterDeath_Event_1`)))
        (:`then_2`
          (add `BaseCharacter.OnCharacterIsDestroy` (delegate `OnCharacterIsDestroy_Event_1`)))
        (:`then_3`
          (add `BaseCharacter.OnCharacterSpawn` (delegate `OnCharacterSpawn_Event_1`)))
        (:`then_4`
          (add `BaseCharacter.OnCharacterTakeLife` (delegate `OnCharacterTakeLife_Event_1`)))))))

(event `OnCharacterTakeDamage_Event_2`
  (params (pBaseCharacter :type "BaseCharacter Object Reference") (RealDamageGive :type "Float (double-precision)") (RealDamageTake :type "Float (double-precision)"))
  ;[1 1 1] Define the Trash behaviours
  (`/Game/Blueprint/Particle/Blood/BloodParticleEmiterComponent.EmiteBloodSplat` (`self.BloodParticleEmiterComponent`)))

(event `OnCharacterDeath_Event_1`
  (params (pBaseCharacter :type "BaseCharacter Object Reference"))
  ;[1 1 1] Define the Trash behaviours
)

(event `OnCharacterIsDestroy_Event_1`
  ;[1 1 1] Define the Trash behaviours
)

(event `OnCharacterSpawn_Event_1`
  ;[1 1 1] Define the Trash behaviours
)

(event `OnCharacterTakeLife_Event_1`
  (params (pBaseCharacter :type "BaseCharacter Object Reference") (RealLifeGive :type "Float (double-precision)") (RealLifeTake :type "Float (double-precision)"))
  ;[1 1 1] Define the Trash behaviours
)

(fn `UserConstructionScript`
  (`parent.UserConstructionScript`))